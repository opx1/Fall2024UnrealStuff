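; MovingBeam is a Blueprint, presumably a moving beam, that travels between three configurable points using an InterpToMovement component.
; The construction script builds the control points, marking the first two locations as relative and leaving the third at the default setting.
; It randomly picks one of three durations for the movement, then restarts it with another random pick from the same values as the argument.
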(fn `UserConstructionScript`
  (bind _interptomovement (`self.InterpToMovement`))
  (bind _outitem (`KismetArrayLibrary.Array_Random` (`|MakeArray` (`self.Duration`) (`self.Duration1`) (`self.Duration2`))))
  (set `InterpToMovementComponent.ControlPoints` (`|MakeArray` (make `InterpControlPoint` (`self.Location 1`)) (make `InterpControlPoint` (`self.Location 2`)) (make `InterpControlPoint` :`PositionControlPoint` (`self.Location 3`))) _interptomovement)
  (set `InterpToMovementComponent.Duration` _outitem _interptomovement)
  (`InterpToMovementComponent.RestartMovement` (`self.InterpToMovement`) _outitem))