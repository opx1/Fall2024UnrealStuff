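; MovingPlatform is a Blueprint actor whose InterpToMovement component moves it along relative control points over a configurable Duration.
; The Construction Script builds the point list from Location1 and Location2, plus a third entry left unconnected, and applies Duration.
; A Location3 point node exists but is not wired into the list.
; The Event Graph holds only disabled stub events, so movement relies entirely on the component.
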(fn `UserConstructionScript`
  (bind _interptomovement (`self.InterpToMovement`))
  (set `InterpToMovementComponent.ControlPoints` (`|MakeArray` (make `InterpControlPoint` (`self.Location 1`)) (make `InterpControlPoint` (`self.Location 2`)) (struct)) _interptomovement)
  (set `InterpToMovementComponent.Duration` (`self.Duration`) _interptomovement))