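; Moving teleporter actor that sends the third-person character to an exit point when it enters the trigger.
; An InterpToMovement component, built in the construction script from three relative locations and a duration, moves the actor and restarts after a pause whenever it stops.
; Exit uses absolute location so it does not follow the moving actor.
; Trigger overlap teleports the character there after a brief delay, with zeroed rotation.
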(event `self.InterpToMovement.OnInterpToStop`
  (params (ImpactResult :type "HitResult Structure (by ref)") (Time :type "Float (single-precision)"))
  (`KismetSystemLibrary.Delay` 3.0)
  (`InterpToMovementComponent.RestartMovement` (`self.InterpToMovement`) 1.0))

(event `self.Trigger.OnComponentBeginOverlap`
  (params (OverlappedComponent :type "PrimitiveComponent Object Reference") (OtherActor :type "Actor Object Reference") (OtherComp :type "PrimitiveComponent Object Reference") (OtherBodyIndex :type Integer) (bFromSweep :type Boolean) (SweepResult :type "HitResult Structure (by ref)"))
  (bind _asbp_third_person_character (cast `/Game/ThirdPerson/Blueprints/BP_ThirdPersonCharacter` OtherActor))
  (`KismetSystemLibrary.Delay` 0.1)
  (`self.K2_TeleportTo` :`self` _asbp_third_person_character :`DestLocation` (`SceneComponent.K2_GetComponentLocation` (`self.Exit`))))

(fn `UserConstructionScript`
  (bind _interptomovement (`self.InterpToMovement`))
  (`SceneComponent.SetAbsolute` (`self.Exit`) true false false)
  (set `InterpToMovementComponent.ControlPoints` (`|MakeArray` (make `InterpControlPoint` (`self.Location 1`)) (make `InterpControlPoint` (`self.Location 2`)) (make `InterpControlPoint` (`self.Location 3`))) _interptomovement)
  (set `InterpToMovementComponent.Duration` (`self.Duration`) _interptomovement))