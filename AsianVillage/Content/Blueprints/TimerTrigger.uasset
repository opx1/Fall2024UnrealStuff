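; TimerTrigger is a Blueprint with two overlap volumes that start and clear an on-screen countdown or timer display.
; Overlapping the Trigger component creates a Timer widget for the first player, passes it the configured minutes and seconds, and adds it to the viewport.
; Overlapping the Exit component removes all widgets, not just the timer.
; Each component disables its collision after firing, so it works once, and neither filters the overlapping actor.
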(event `self.Trigger.OnComponentBeginOverlap`
  (params (OverlappedComponent :type "PrimitiveComponent Object Reference") (OtherActor :type "Actor Object Reference") (OtherComp :type "PrimitiveComponent Object Reference") (OtherBodyIndex :type Integer) (bFromSweep :type Boolean) (SweepResult :type "HitResult Structure (by ref)"))
  (bind _returnvalue (`|CreateWidget` "/Game/Blueprints/Timer.Timer_C" (`GameplayStatics.GetPlayerController` 0)))
  (set `/Game/Blueprints/Timer.Minutes` (`self.MinutesSet`) _returnvalue)
  (set `/Game/Blueprints/Timer.Seconds` (`self.SecondsSet`) _returnvalue)
  (`UserWidget.AddToViewport` _returnvalue 0)
  (`PrimitiveComponent.SetCollisionEnabled` (`self.Trigger`) "NoCollision"))

(event `self.Exit.OnComponentBeginOverlap`
  (params (OverlappedComponent :type "PrimitiveComponent Object Reference") (OtherActor :type "Actor Object Reference") (OtherComp :type "PrimitiveComponent Object Reference") (OtherBodyIndex :type Integer) (bFromSweep :type Boolean) (SweepResult :type "HitResult Structure (by ref)"))
  (`WidgetLayoutLibrary.RemoveAllWidgets`)
  (`PrimitiveComponent.SetCollisionEnabled` (`self.Exit`) "NoCollision"))

(fn `UserConstructionScript`)